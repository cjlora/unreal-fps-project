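; Parasol prop Blueprint from the procedural building generator that varies its look by picking materials from an array.
; The construction script randomizes two seeds and derives an independent material index for each of the two rubber slots on the parasol.
; An executed flag keeps the picks stable across construction reruns, while a RandomizeMaterial toggle triggers a reroll and then resets itself.
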(event EventBeginPlay)

(event Collision|EventActorBeginOverlap
  (params (OtherActor :type Actor%20Object%20Reference)))

(event EventTick
  (params (DeltaSeconds :type Float%20%28single-precision%29)))

(fn ConstructionScript
  (bind _parasol (Variables|Default|GetParasol))
  (if (> (Utilities|Array|Length (Variables|Default|GetMaterial)) 0)
    (Utilities|FlowControl|Sequence
      (:then_0
        (if (or (Variables|Default|GetRandomize%20material) (not (Variables|Default|GetAlready%20Executed)))
          (Class|KismetMathLibrary|SeedRandomStream (Variables|Default|GetSeed))
          (Class|KismetMathLibrary|SeedRandomStream (Variables|Default|GetSeed%201))
          (Variables|Default|SetMaterial%20ID (Math|Random|RandomIntegerinRangefromStream 0 (- (Utilities|Array|Length (Variables|Default|GetMaterial)) 1) (Math|Random|MakeRandomStream (.initialseed (Variables|Default|GetSeed)))))
          (Variables|Default|SetMaterial%20ID%201 (Math|Random|RandomIntegerinRangefromStream 0 (- (Utilities|Array|Length (Variables|Default|GetMaterial)) 1) (Math|Random|MakeRandomStream (.initialseed (Variables|Default|GetSeed%201)))))))
      (:then_1
        (Rendering|Material|SetMaterialbyName _parasol "Rubber_1" (Utilities|Array|Get(acopy) (Variables|Default|GetMaterial) (Variables|Default|GetMaterial%20ID)))
        (Rendering|Material|SetMaterialbyName _parasol "Rubber_2" (Utilities|Array|Get(acopy) (Variables|Default|GetMaterial) (Variables|Default|GetMaterial%20ID%201))))
      (:then_2
        (Variables|Default|SetAlready%20Executed true)
        (Variables|Default|SetRandomize%20material false)))))